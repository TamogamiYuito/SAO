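; VR player character that sets up headset tracking, input and hand actors on BeginPlay.
; With an HMD enabled, it sets floor-level tracking, adjusts the secondary-screen render target percentage, adds the default and hand Enhanced Input contexts, then hides the loading screen.
; Regardless of HMD state, it spawns separate left and right hand actors, owned by itself and snapped to its Origin component.
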(event EventBeginPlay
  (bind _returnvalue (Game|GetPlayerController 0))
  (bind _self self)
  (bind _returnvalue_2 (PlayerController|LocalPlayerSubsystems|GetEnhancedInputLocalPlayerSubsystem _returnvalue))
  (Utilities|FlowControl|Sequence
    (:then_0
      (if (Class|HeadMountedDisplayFunctionLibrary|IsHeadMountedDisplayEnabled)
        (Utilities|FlowControl|Sequence
          (:then_0
            (Class|HeadMountedDisplayFunctionLibrary|SetTrackingOrigin "LocalFloor")
            (Development|ExecuteConsoleCommand "xr.SecondaryScreenPercentage.HMDRenderTarget 100" 0)
            (Input|AddMappingContext _returnvalue_2 "/Game/XRFramework/Input/IMC_Default.IMC_Default" 0 "(bIgnoreAllPressedKeysUntilRelease=True,bForceImmediately=False,bNotifyUserSettings=False)")
            (Input|AddMappingContext _returnvalue_2 "/Game/XRFramework/Input/IMC_Hands.IMC_Hands" 0 "(bIgnoreAllPressedKeysUntilRelease=True,bForceImmediately=False,bNotifyUserSettings=False)"))
          (:then_1
            (Class|XRLoadingScreenFunctionLibrary|HideLoadingScreen)))))
    (:then_1
      (Utilities|FlowControl|Sequence
        (:then_0
          (bind _returnvalue_3 (Game|SpawnActorfromClass "/Game/BP_LeftHand.BP_LeftHand_C" (Math|Transform|MakeTransform "0, 0, 0" "0, 0, 0" "1.000000,1.000000,1.000000") "Undefined" "MultiplyWithRoot" _self 0))
          (Transformation|AttachComponentToComponent _returnvalue_3 (Variables|Default|GetOrigin) "None" "SnapToTarget" "SnapToTarget" "KeepWorld" true))
        (:then_1
          (bind _returnvalue_4 (Game|SpawnActorfromClass "/Game/BP_RightHand.BP_RightHand_C" (Math|Transform|MakeTransform "0, 0, 0" "0, 0, 0" "1.000000,1.000000,1.000000") "Undefined" "MultiplyWithRoot" _self 0))
          (Transformation|AttachComponentToComponent _returnvalue_4 (Variables|Default|GetOrigin) "None" "SnapToTarget" "SnapToTarget" "KeepWorld" true))))))

(fn ConstructionScript)